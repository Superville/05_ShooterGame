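; AI controller for guard NPCs that runs the GuardBehavior tree on the PatrolData blackboard.
; Perception sets or clears the blackboard enemy key as it senses or loses living GuardPawn_BP actors without the Guard tag.
; Each tick, the controlled pawn's Aiming and Shooting flags follow whether a valid focus actor exists; despite its name, SetAimingPitch computes no pitch.
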(event OnTargetPerceptionUpdated(AIPerception)
  (params (Actor :type Actor%20Object%20Reference) (Stimulus :type AI%20Stimulus%20Structure))
  (bind _enemykey (Variables|Default|GetEnemyKey))
  (bind _blackboardcomp (Variables|Default|GetBlackboardComp))
  (bind _asguard_pawn_bp (Utilities|Casting|CastToGuardPawn_BP Actor))
  (if (not (or (Actor|ActorHasTag Actor "Guard") (Default|IsDead _asguard_pawn_bp)))
    (if (.bSuccessfullySensed (Utilities|Struct|BreakAIStimulus Stimulus))
      (AI|Components|Blackboard|SetValueasObject _blackboardcomp _enemykey Actor)
      (else
        (AI|Components|Blackboard|ClearValue _blackboardcomp _enemykey)))))

(event EventBeginPlay
  (bind _blackboardcomponent (Class|AIController|UseBlackboard "/Game/Dynamic/Characters/NPC/AI/PatrolData.PatrolData"))
  (AI|RunBehaviorTree "/Game/Dynamic/Characters/NPC/AI/GuardBehavior.GuardBehavior")
  (Variables|Default|SetBlackboardComp _blackboardcomponent)
  (bind _asguard_pawn_bp (Utilities|Casting|CastToGuardPawn_BP (Pawn|GetControlledPawn)))
  (Variables|Default|SetMyPawn _asguard_pawn_bp))

(event EventTick
  (params (DeltaSeconds :type Float%20%28single-precision%29))
  (bind _output_get (CallFunction|SetAimingPitch))
  (Variables|/Game/Dynamic/Characters/NPC/Blueprints/GuardPawn_BP.GuardPawn_BP_C|SetShooting (Variables|Default|GetMyPawn) _output_get))

(fn ConstructionScript)

(fn SetAimingPitch
  (bind _output_get (Variables|/Game/Dynamic/Characters/NPC/Blueprints/GuardPawn_BP.GuardPawn_BP_C|SetAiming (Variables|Default|GetMyPawn) (Utilities|IsValid (Class|AIController|GetFocusActor))))
  (return _output_get))