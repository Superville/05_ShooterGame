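; AI controller for guard NPCs that runs the guard behavior tree on patrol blackboard data and tracks a perceived enemy.
; Perception updates set the blackboard enemy key when a valid target is sensed and clear it when that target is lost.
; Valid targets are living BP_GuardPawn actors without the Guard tag; dead targets are ignored entirely, so their updates never clear the key.
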(event OnTargetPerceptionUpdated(AIPerception)
  (params (Actor :type Actor%20Object%20Reference) (Stimulus :type AI%20Stimulus%20Structure))
  (CallFunction|UpdateBlackboardEnemyKey Actor Stimulus))

(event EventBeginPlay
  (bind _blackboardcomponent (Class|AIController|UseBlackboard "/Game/Dynamic/Characters/Guard/AI/BB_PatrolData.BB_PatrolData"))
  (AI|RunBehaviorTree "/Game/Dynamic/Characters/Guard/AI/BT_GuardBehavior.BT_GuardBehavior")
  (Variables|Default|SetBlackboardComp _blackboardcomponent))

(fn ConstructionScript)

(fn UpdateBlackboardEnemyKey
  (params (Actor :type Actor%20Object%20Reference) (AIStimulus :type AI%20Stimulus%20Structure%20%28by%20ref%29))
  (bind _output_get (LocalVariables|SetInputActor Actor))
  (bind _asbp_guard_pawn (Utilities|Casting|CastToBP_GuardPawn _output_get))
  (if (CallFunction|IsValidTarget _asbp_guard_pawn)
    (if (.bSuccessfullySensed (Utilities|Struct|BreakAIStimulus AIStimulus))
      (AI|Components|Blackboard|SetValueasObject (Variables|Default|GetBlackboardComp) (Variables|Default|GetEnemyKey) (LocalVariables|GetInputActor))
      (else
        (AI|Components|Blackboard|ClearValue (Variables|Default|GetBlackboardComp) (Variables|Default|GetEnemyKey))))))

(fn IsValidTarget
  (params (Target :type BP%20Guard%20Pawn%20Object%20Reference))
  (return (not (or (Actor|ActorHasTag Target "Guard") (Class|ThirdPersonCharacter|IsDead Target)))))