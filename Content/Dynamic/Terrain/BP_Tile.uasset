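; Terrain tile for an infinite-terrain mode that scatters random props between two bound markers on BeginPlay and exposes an arrow transform as an attach point.
; A player-tracking box unlocks the barrier while the player overlaps it, toggling collision and red/green material.
; When the player enters the self-destruct box, the tile asks BP_InfiniteTerrainGameMode to spawn another tile, then destroys itself.
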(event OnComponentEndOverlap(TrackPlayerBox)
  (params (OverlappedComponent :type Primitive%20Component%20Object%20Reference) (OtherActor :type Actor%20Object%20Reference) (OtherComp :type Primitive%20Component%20Object%20Reference) (OtherBodyIndex :type Integer))
  (Utilities|IsPlayerActor OtherActor)
  (CallFunction|LockBarrier))

(event OnComponentBeginOverlap(SelfDestructBox)
  (params (OverlappedComponent :type Primitive%20Component%20Object%20Reference) (OtherActor :type Actor%20Object%20Reference) (OtherComp :type Primitive%20Component%20Object%20Reference) (OtherBodyIndex :type Integer) (bFromSweep :type Boolean) (SweepResult :type Hit%20Result%20Structure%20%28by%20ref%29))
  (Utilities|IsPlayerActor OtherActor)
  (bind _asbp_infinite_terrain_game_mode (Utilities|Casting|CastToBP_InfiniteTerrainGameMode (Game|GetGameMode)))
  (Default|SpawnTile _asbp_infinite_terrain_game_mode)
  (Actor|DestroyActor))

(event OnComponentBeginOverlap(TrackPlayerBox)
  (params (OverlappedComponent :type Primitive%20Component%20Object%20Reference) (OtherActor :type Actor%20Object%20Reference) (OtherComp :type Primitive%20Component%20Object%20Reference) (OtherBodyIndex :type Integer) (bFromSweep :type Boolean) (SweepResult :type Hit%20Result%20Structure%20%28by%20ref%29))
  (Utilities|IsPlayerActor OtherActor)
  (CallFunction|UnlockBarrier))

(event EventBeginPlay
  (CallFunction|LockBarrier)
  (Class|Tile|SpawnActorsWithinTile (Transformation|GetWorldLocation (Variables|Default|GetFBox_Min)) (Transformation|GetWorldLocation (Variables|Default|GetFBox_Max)) (Variables|Default|GetPropClasses) 5 20))

(event Collision|EventActorBeginOverlap
  (params (OtherActor :type Actor%20Object%20Reference)))

(event EventTick
  (params (DeltaSeconds :type Float%20%28single-precision%29)))

(fn ConstructionScript)

(fn GetAttachLocation
  (return (Transformation|GetWorldTransform (Variables|Default|GetArrow))))

(fn UnlockBarrier
  (Collision|SetCollisionEnabled (Variables|Default|GetBarrier) "NoCollision")
  (Rendering|Material|SetMaterial (Variables|Default|GetBarrier) 0 "/Game/Dynamic/Terrain/MI_Barrier_Green.MI_Barrier_Green"))

(fn LockBarrier
  (Collision|SetCollisionEnabled (Variables|Default|GetBarrier) "QueryAndPhysics")
  (Rendering|Material|SetMaterial (Variables|Default|GetBarrier) 0 "/Game/Dynamic/Terrain/MI_Barrier_Red.MI_Barrier_Red"))