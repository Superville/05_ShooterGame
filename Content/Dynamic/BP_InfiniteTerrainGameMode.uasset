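; Game mode for an infinite terrain game that lays the initial run of tiles on BeginPlay and tracks the player's score.
; It starts from the placed tile tagged StartTile, then chains BP_Tile spawns by placing each at the previous tile's attach location.
; It fills a NavMeshBoundsVolume pool first and hands it to every spawned tile.
; Helper functions increment the score and format it as a display string.
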(event EventBeginPlay
  (Class|InfiniteTerrainGameMode|PopulateNavMeshBoundsVolumePool)
  (CallFunction|SpawnTiles 4))

(fn ConstructionScript)

(fn SpawnTiles
  (params (NumTiles :type Integer))
  (CallFunction|FindStartTile)
  (for _index (range 0 (- NumTiles 1))
    (CallFunction|SpawnTile)))

(fn SpawnTile
  (bind _returnvalue (Game|SpawnActorfromClass "/Game/Dynamic/Terrain/BP_Tile.BP_Tile_C" (Variables|Default|GetNextTileTransform) "Undefined" 0 0))
  (Class|Tile|SetActorPool _returnvalue (Variables|Default|GetNavMeshBoundsVolumePool))
  (Variables|Default|SetNextTileTransform (Default|GetAttachLocation _returnvalue)))

(fn RecordPlayerScore
  (Math|Integer|IncrementInt (Variables|Default|GetScore)))

(fn GetScoreString
  (return (Utilities|String|Append "Score: " (Utilities|String|ToString(Integer) (Variables|Default|GetScore)))))

(fn FindStartTile
  (bind _outactors (Actor|GetAllActorsOfClass "/Game/Dynamic/Terrain/BP_Tile.BP_Tile_C"))
  (for _array_element _outactors
    (if (Actor|ActorHasTag _array_element "StartTile")
      (Variables|Default|SetNextTileTransform (Default|GetAttachLocation _array_element)))))